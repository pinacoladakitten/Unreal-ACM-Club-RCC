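; BP_Finish is a level-exit actor that loads the next level when the player's pawn overlaps it.
; On overlap it looks up the current level name in the Levels array held by BP_NewGameMode and increments that index.
; It opens the level at the resulting index by name, wrapping to the first entry after the last one.
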(event `self.ReceiveActorBeginOverlap`
  (params (OtherActor :type "Actor Object Reference"))
  (if (== OtherActor (`GameplayStatics.GetPlayerPawn` 0))
    (bind _asbp_new_game_mode (cast `/Game/Game/BP_NewGameMode` (`GameplayStatics.GetGameMode`)))
    (bind _returnvalue (`GameplayStatics.GetCurrentLevelName` true))
    (bind _levels (`/Game/Game/BP_NewGameMode.Levels` _asbp_new_game_mode))
    (bind _result (`/Engine/EditorBlueprintResources/StandardMacros.IncrementInt` (`KismetArrayLibrary.Array_Find` _levels _returnvalue))
      (:`  `
        (if (>= _result (`KismetArrayLibrary.Array_Length` _levels))
          (`GameplayStatics.OpenLevel` (`KismetStringLibrary.Conv_StringToName` (`|GetArrayItem` _levels)))
          (else
            (`GameplayStatics.OpenLevel` (`KismetStringLibrary.Conv_StringToName` (`|GetArrayItem` _levels _result)))))))))

(fn `UserConstructionScript`)