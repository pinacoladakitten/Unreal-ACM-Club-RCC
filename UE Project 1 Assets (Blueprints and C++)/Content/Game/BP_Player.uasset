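; BP_Player is a player actor with a Cube component that returns to its starting position when it hits an obstacle.
; BeginPlay caches the start location, and an overlap with an actor of class BP_obstacle teleport-free resets the actor to it, printing a debug True or False for each overlap.
; Force-based movement from the horizontal and vertical input axes exists but is disconnected, so it never runs.
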(event `self.ReceiveBeginPlay`
  (set `self.StartLocation` (`self.K2_GetActorLocation`)))

(event `self.ReceiveTick`
  (params (DeltaSeconds :type "Float (single-precision)")))

(event `self.ReceiveActorBeginOverlap`
  (params (OtherActor :type "Actor Object Reference"))
  (if (== (`GameplayStatics.GetObjectClass` OtherActor) "/Game/Game/BP_obstacle.BP_obstacle_C")
    (`KismetSystemLibrary.PrintString` "True")
    (`self.K2_SetActorLocation` (`self.StartLocation`))
    (else
      (`KismetSystemLibrary.PrintString` "False"))))

(fn `UserConstructionScript`)