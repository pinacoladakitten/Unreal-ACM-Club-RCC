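; BP_Player is a player Blueprint that moves a Cube component by applying physics forces from horizontal and vertical movement input.
; Each Tick scales both input values by Speed and feeds them into AddForce on X and Y, with the vertical value negated.
; BeginPlay stores the actor's starting location, which these graphs never read.
; A Camera forward-vector node is left unused, so movement ignores camera orientation.
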(event `self.ReceiveBeginPlay`
  (set `self.StartLocation` (`self.K2_GetActorLocation`)))

(event `self.ReceiveTick`
  (params (DeltaSeconds :type "Float (single-precision)"))
  (`PrimitiveComponent.AddForce` (`self.Cube`) (`KismetMathLibrary.MakeVector` (* (`self.GetInputAxisValue`) (`self.Speed`)) (* (`self.GetInputAxisValue`) (`self.Speed`) -1.0)) "None" false))

(fn `UserConstructionScript`)